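; BP_CompleteCarBasic is a subway car that leapfrogs with a linked PreviousCar as the player advances.
; On BeginPlay it optionally spawns its interior actor, then enables enemy spawning for later interiors, and assigns the left and right track child actors to its wall scenery.
; When the player overlaps the shuffle trigger, it teleports PreviousCar to the attach point and spawns a new interior there, passing the enemy flag.
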(event OnComponentBeginOverlap(ShuffleNewCarTrigger)
  (params (OverlappedComponent :type Primitive%20Component%20Object%20Reference) (OtherActor :type Actor%20Object%20Reference) (OtherComp :type Primitive%20Component%20Object%20Reference) (OtherBodyIndex :type Integer) (bFromSweep :type Boolean) (SweepResult :type Hit%20Result%20Structure%20%28by%20ref%29))
  (Utilities|Casting|CastToBP_PlayerShooterCharacter OtherActor)
  (Transformation|SetActorLocation (Variables|Default|GetPreviousCar) (Transformation|GetWorldLocation (Variables|Default|GetNewCarAttach)) false true)
  (bind _interior (CallFunction|SetUpCar (Variables|Default|GetPreviousCar)))
  (Variables|Default|SetNewCarInterior _interior))

(event EventBeginPlay
  (if (Variables|Default|GetSpawnInterior)
    (bind _interior (CallFunction|SetUpCar self))
    (Variables|Default|SetNewCarInterior _interior)
    (Variables|Default|SetSpawnEnemies true))
  (bind _asbp_scenery (Utilities|Casting|CastToBP_Scenery (Variables|/Script/Engine.ChildActorComponent|GetChildActor (Variables|Default|GetSubwayWall_1))))
  (bind _asbp_scenery_track (Utilities|Casting|CastToBP_SceneryTrack (Variables|/Script/Engine.ChildActorComponent|GetChildActor (Variables|Default|GetMovementTrackLeft))))
  (Variables|/Game/Game/Blueprints/BP_Scenery.BP_Scenery_C|SetTrack _asbp_scenery _asbp_scenery_track)
  (bind _asbp_scenery_2 (Utilities|Casting|CastToBP_Scenery (Variables|/Script/Engine.ChildActorComponent|GetChildActor (Variables|Default|GetSubwayWall_2))))
  (bind _asbp_scenery_track_2 (Utilities|Casting|CastToBP_SceneryTrack (Variables|/Script/Engine.ChildActorComponent|GetChildActor (Variables|Default|GetMovementTrackRight))))
  (Variables|/Game/Game/Blueprints/BP_Scenery.BP_Scenery_C|SetTrack _asbp_scenery_2 _asbp_scenery_track_2))

(fn ConstructionScript)

(fn SetUpCar
  (params (Car :type Actor%20Object%20Reference))
  (bind _returnvalue (Game|SpawnActorfromClass "/Game/Game/Blueprints/BP_CompleteCarInterior.BP_CompleteCarInterior_C" (Transformation|GetActorTransform Car) "AdjustIfPossibleButAlwaysSpawn" self (Variables|Default|GetSpawnEnemies) 0))
  (return _returnvalue))

(fn SetUpSceneryTrack
  (params (Scenery :type BP%20Scenery%20Object%20Reference) (Track :type BP%20Scenery%20Track%20Object%20Reference)))