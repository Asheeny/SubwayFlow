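; BP_SM_door_end_01_DM is a destructible end door that shatters when the player approaches and counts toward level progress.
; Entering its trigger enables physics for any actor; for the player it also sets InRangeOfDoor, applies radius damage and force at Impact, and ignores two custom collision channels.
; When the player leaves, it clears that flag, increments CarsCleared on the first BP_LevelTracker found, and destroys itself after a short delay.
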(event OnComponentEndOverlap(EnterTriggerVolume)
  (params (OverlappedComponent :type Primitive%20Component%20Object%20Reference) (OtherActor :type Actor%20Object%20Reference) (OtherComp :type Primitive%20Component%20Object%20Reference) (OtherBodyIndex :type Integer))
  (bind _asbp_player_shooter_character (Utilities|Casting|CastToBP_PlayerShooterCharacter OtherActor))
  (Variables|/Script/SimpleShooter.ShooterCharacter|SetbInRangeOfDoor _asbp_player_shooter_character false)
  (bind _outactors (Actor|GetAllActorsOfClass "/Game/Game/Blueprints/BP_LevelTracker.BP_LevelTracker_C"))
  (Variables|/Game/Game/Blueprints/BP_LevelTracker.BP_LevelTracker_C|SetCarsCleared (Utilities|Array|Get(acopy) _outactors) (+ (Variables|/Game/Game/Blueprints/BP_LevelTracker.BP_LevelTracker_C|GetCarsCleared (Utilities|Array|Get(acopy) _outactors)) 1))
  (Utilities|FlowControl|Delay 0.2)
  (Actor|DestroyActor))

(event OnComponentBeginOverlap(EnterTriggerVolume)
  (params (OverlappedComponent :type Primitive%20Component%20Object%20Reference) (OtherActor :type Actor%20Object%20Reference) (OtherComp :type Primitive%20Component%20Object%20Reference) (OtherBodyIndex :type Integer) (bFromSweep :type Boolean) (SweepResult :type Hit%20Result%20Structure%20%28by%20ref%29))
  (bind _destructible (Variables|Default|GetDestructible))
  (bind _destructible_2 (Variables|Default|GetDestructible))
  (bind _destructible_3 (Variables|Default|GetDestructible))
  (bind _impact (Variables|Default|GetImpact))
  (bind _returnvalue (Transformation|GetWorldLocation _impact))
  (Physics|SetSimulatePhysics _destructible_2 true)
  (Physics|SetEnableGravity _destructible_2 true)
  (bind _asbp_player_shooter_character (Utilities|Casting|CastToBP_PlayerShooterCharacter OtherActor))
  (Variables|/Script/SimpleShooter.ShooterCharacter|SetbInRangeOfDoor _asbp_player_shooter_character true)
  (Class|DestructibleComponent|ApplyRadiusDamage _destructible_3 1e+03 _returnvalue 2.5e+03 1e+04 false)
  (Physics|AddRadialForce _destructible_3 _returnvalue 2e+02 1e+04 "RIF_Constant" false)
  (Collision|SetCollisionResponsetoChannel _destructible "ECC_GameTraceChannel1" "ECR_Ignore")
  (Collision|SetCollisionResponsetoChannel _destructible "ECC_GameTraceChannel2" "ECR_Ignore"))

(fn ConstructionScript)