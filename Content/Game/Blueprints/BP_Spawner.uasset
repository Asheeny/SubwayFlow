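; BP_Spawner is a scene component that may spawn an actor of a configurable class at its own world transform.
; On BeginPlay it rolls a random float against ChanceToSpawn, then waits SpawnDelay before a single spawn.
; The spawned actor takes the component's owner as its Owner and gets a life span from Lifetime.
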(event EventBeginPlay
  (if (< (Math|Random|RandomFloatinRange 0.0 1.0) (Variables|Default|GetChanceToSpawn))
    (Utilities|FlowControl|Delay (Variables|Default|GetSpawnDelay))
    (bind _returnvalue (Game|SpawnActorfromClass (Variables|Default|GetToSpawn) (Transformation|GetWorldTransform) "Undefined" (Components|GetOwner self) 0))
    (Actor|SetLifeSpan _returnvalue (Variables|Default|GetLifetime))))