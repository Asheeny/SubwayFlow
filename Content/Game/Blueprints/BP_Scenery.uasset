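; BP_Scenery is a scenery actor with two lamps that travels along the spline of a referenced Track.
; On BeginPlay it gives each lamp a random colour from LightColours and starts the TrackMovement timeline at a randomised play rate, so travel speed varies between instances.
; Each timeline update maps Position to distance along the spline and moves the actor there in world space, keeping its current rotation.
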(event EventBeginPlay
  (bind _returnvalue (Transformation|GetActorRotation))
  (bind _track (Variables|Default|GetTrack))
  (bind _spline (Variables|/Game/Game/Blueprints/BP_SceneryTrack.BP_SceneryTrack_C|GetSpline _track))
  (CallFunction|SetRandomLightColour (Variables|Default|GetLamp))
  (CallFunction|SetRandomLightColour (Variables|Default|GetLamp1))
  (Components|Timeline|SetPlayRate (Variables|Default|GetTrackMovement) (/ 1.0 (Math|Random|RandomFloatinRange 3.0 4.0)))
  (bind _position (Timeline|TrackMovement Play)
    (:Update
      (Transformation|SetActorLocationAndRotation (Spline|GetLocationatDistanceAlongSpline _spline (Math|Float|Lerp 0.0 (Spline|GetSplineLength _spline) _position) "World") (Math|Rotator|MakeRotator (.roll _returnvalue) (.pitch _returnvalue) (.yaw _returnvalue))))))

(fn ConstructionScript)

(fn SetRandomLightColour
  (params (Light :type Light%20Component%20Object%20Reference))
  (bind _lightcolours (Variables|Default|GetLightColours))
  (Rendering|Components|Light|SetLightColor Light (Utilities|Array|Get(acopy) _lightcolours (Math|Random|RandomIntegerinRange 0 (- (Utilities|Array|Length _lightcolours) 1))) true))