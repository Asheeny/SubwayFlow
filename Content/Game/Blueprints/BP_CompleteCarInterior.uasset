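; BP_CompleteCarInterior is a car interior actor with five enemy spawners and a link to the car before it.
; Its construction script gathers the spawners into an array and zeroes their spawn chance when enemy spawning is disabled.
; An optional flag gives the actor a short fixed lifespan at BeginPlay.
; SetPreviousCar stores the reference to the preceding car, which this Blueprint does not otherwise use.
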(event EventBeginPlay
  (if (Variables|Default|GetSetLifeTime)
    (Actor|SetLifeSpan 15.0)))

(fn ConstructionScript
  (Variables|Default|SetSpawnPoints (Utilities|Array|MakeArray (Variables|Default|GetSpawner1) (Variables|Default|GetSpawner2) (Variables|Default|GetSpawner3) (Variables|Default|GetSpawner4) (Variables|Default|GetSpawner5)))
  (if (not (Variables|Default|GetSpawnEnemeis))
    (for _array_element (Variables|Default|GetSpawnPoints)
      (Variables|/Game/Game/Blueprints/BP_Spawner.BP_Spawner_C|SetChanceToSpawn _array_element 0.0))))

(fn SetPreviousCar
  (params (PreviousCarRef :type Actor%20Object%20Reference))
  (Variables|Default|SetPreviousCar PreviousCarRef))