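; Player shooter character that moves automatically along world negative X and slows time when in range of a door.
; Each tick applies movement input at a scale initialized from the base value, then branches on the door-range flag.
; Begin and end slow-mo timelines blend global time dilation toward the slow maximum or normal speed.
; Their updates drive a vision-ease timeline in reverse or forward, feeding a material parameter collection.
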(event EventBeginPlay
  (|CallParentFunction) ; This node is disabled and will not be called.\nDrag off pins to build functionality.
)

(event Collision|EventActorBeginOverlap
  (params (OtherActor :type Actor%20Object%20Reference))
  (|CallParentFunction OtherActor) ; This node is disabled and will not be called.\nDrag off pins to build functionality.
)

(event EventTick
  (params (DeltaSeconds :type Float%20%28single-precision%29))
  (|CallParentFunction DeltaSeconds)
  (Pawn|Input|AddMovementInput (* (Class|KismetMathLibrary|VectorForward) -1) (Variables|Default|GetCurrentMovementScale) false)
  (if (Variables|Default|GetbInRangeOfDoor)
    (bind _rate (Timeline|BeginSlowMo Play)
      (:Update
        (Utilities|Time|SetGlobalTimeDilation (Math|Float|Lerp (Class|GameplayStatics|GetGlobalTimeDilation) (Variables|Default|GetSlowMoMax) _rate))
        (bind _rate_2 (Timeline|VisionEase ReverseFromEnd)
          (:Update
            (Rendering|Material|SetScalarParameterValue "/Game/Materials/PC_Vision.PC_Vision" "VisionEaseRate" _rate_2 :!class /Script/Engine.KismetMaterialLibrary)))))
    (else
      (bind _rate_3 (Timeline|EndSlowMo Play)
        (:Update
          (Utilities|Time|SetGlobalTimeDilation (Math|Float|Lerp (Class|GameplayStatics|GetGlobalTimeDilation) 1.0 _rate_3))
          (Timeline|VisionEase PlayFromStart))))))

(fn ConstructionScript
  (|CallParentFunction)
  (Variables|Default|SetCurrentMovementScale (Variables|Default|GetBaseMovementScale)))