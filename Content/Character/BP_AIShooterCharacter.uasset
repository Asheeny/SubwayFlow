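; AI-controlled shooter character Blueprint that dies on contact with the player and deals impact damage in return.
; On capsule overlap while alive, it flags the player as in melee range and takes damage equal to its own current health, credited to the player.
; It then damages the player by ImpactDamagePercent of their current health.
; Ending the overlap clears the player's melee-range flag.
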(event OnComponentBeginOverlap(CapsuleComponent)
  (params (OverlappedComponent :type Primitive%20Component%20Object%20Reference) (OtherActor :type Actor%20Object%20Reference) (OtherComp :type Primitive%20Component%20Object%20Reference) (OtherBodyIndex :type Integer) (bFromSweep :type Boolean) (SweepResult :type Hit%20Result%20Structure%20%28by%20ref%29))
  (bind _self self)
  (if (not (Class|ShooterCharacter|IsDead))
    (bind _asbp_player_shooter_character (Utilities|Casting|CastToBP_PlayerShooterCharacter OtherActor))
    (Variables|/Script/SimpleShooter.ShooterCharacter|SetbInMeleeRange _asbp_player_shooter_character true)
    (Class|ShooterCharacter|TakeDamage (Variables|Default|GetCurrentHealth) (Utilities|Struct|MakeDamageEvent) (Pawn|GetController _asbp_player_shooter_character) _asbp_player_shooter_character)
    (Class|ShooterCharacter|TakeDamage _asbp_player_shooter_character (* (Variables|/Script/SimpleShooter.ShooterCharacter|GetCurrentHealth _asbp_player_shooter_character) (Variables|Default|GetImpactDamagePercent)) (Utilities|Struct|MakeDamageEvent) (Pawn|GetController _self) _self)))

(event OnComponentEndOverlap(CapsuleComponent)
  (params (OverlappedComponent :type Primitive%20Component%20Object%20Reference) (OtherActor :type Actor%20Object%20Reference) (OtherComp :type Primitive%20Component%20Object%20Reference) (OtherBodyIndex :type Integer))
  (bind _asbp_player_shooter_character (Utilities|Casting|CastToBP_PlayerShooterCharacter OtherActor))
  (Variables|/Script/SimpleShooter.ShooterCharacter|SetbInMeleeRange _asbp_player_shooter_character false))

(event EventBeginPlay
  (|CallParentFunction) ; This node is disabled and will not be called.\nDrag off pins to build functionality.
)

(event EventTick
  (params (DeltaSeconds :type Float%20%28single-precision%29))
  (|CallParentFunction DeltaSeconds) ; This node is disabled and will not be called.\nDrag off pins to build functionality.
)

(fn ConstructionScript
  (|CallParentFunction))